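; BP_Grid is a grid Blueprint that routes selection events from its cells back to itself.
; On BeginPlay it loops over GridCells, casts each to BP_Cell and binds its cell-selected event to a custom event that calls SelectCell.
; Debug prints mark startup and the end of binding.
; Bindings for grid-initialized and select events are left unconnected, and construction and destruction logic are empty.
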(event `OnGridInitialized_Event`)

(event `self.ReceiveBeginPlay`
  (`KismetSystemLibrary.PrintString` "BeginPlay")
  (for _array_element (`self.GridCells`)
    (cast `/Game/Grid/BP_Cell` _array_element)
    (add `Cell.OnCellSelected` _array_element (delegate `CustomEvent`)))
  (`KismetSystemLibrary.PrintString` "Cells bounded"))

(event `CustomEvent`
  (params (SelectedCell :type "Cell Object Reference"))
  (`self.SelectCell` SelectedCell))

(event `self.ReceiveDestroyed`)

(event `OnCellSelected_Event`
  (params (NewParam :type "Cell Object Reference"))
  (`KismetSystemLibrary.PrintString` "Select Cell"))

(fn `UserConstructionScript`)